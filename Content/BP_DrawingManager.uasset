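; Drawing manager actor that records a freehand mouse stroke in the world as a spline.
; BeginPlay shows the cursor in game-and-UI mode; holding left mouse clears DrawingSpline and enables drawing.
; While drawing, Tick adds a spline point at the Visibility trace hit under the cursor and marks it with a short-lived red debug sphere.
; UpdateSplineMesh is empty, and StartDrawing, StopDrawing and EnableInput sit only in unconnected logic.
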(event `self.ReceiveBeginPlay`
  (bind _returnvalue (`GameplayStatics.GetPlayerController` 0))
  (`WidgetBlueprintLibrary.SetInputMode_GameAndUIEx` _returnvalue null "DoNotLock" false)
  (set `PlayerController.bShowMouseCursor` true _returnvalue)
  (`Controller.ResetIgnoreLookInput` _returnvalue))

(event `self.ReceiveTick`
  (params (DeltaSeconds :type "Float (single-precision)"))
  (bind (_bblockinghit _binitialoverlap _time _distance _location) (`GameplayStatics.BreakHitResult` (`PlayerController.GetHitResultUnderCursorByChannel` (`GameplayStatics.GetPlayerController` 0) "TraceTypeQuery1" false)))
  (if (`self.bIsDrawing`)
    (`|ExecutionSequence`
      (:`then_0`
        (`KismetSystemLibrary.DrawDebugSphere` _location 20.0 12 (struct :`R` 1.0 :`G` 0.022917 :`B` 0.022917 :`A` 1.0) 0.5))
      (:`then_1`
        (`SplineComponent.AddSplinePoint` (`self.DrawingSpline`) _location "World" true)))))

(event `Key|LeftMouseButton`
  (params (Key :type "Key Structure"))
  (:`Pressed`
    (`|ExecutionSequence`
      (:`then_0`
        (`SplineComponent.ClearSplinePoints` (`self.DrawingSpline`) true))
      (:`then_1`
        (set `self.bIsDrawing` true))))
  (:`Released`
    (set `self.bIsDrawing` false)))

(fn `StartDrawing`
  (`KismetSystemLibrary.PrintString` "StarDrawing")
  (set `self.bIsDrawing` true)
  (`SplineComponent.ClearSplinePoints` (`self.DrawingSpline`) true)
  (`KismetSystemLibrary.PrintString` "clear"))

(fn `StopDrawing`
  (set `self.bIsDrawing` false))

(fn `UpdateSplineMesh`)

(fn `UserConstructionScript`)