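; AC_PlantSpawner scatters plant mesh instances along a given spline.
; GeneratePlants steps along the spline at SpawnSpacing and adds an instance to InstancedMeshComponent with random yaw and random per-axis scale.
; Base rotation derives from the spline point's world location rather than its direction, and world-space locations are passed as component-local transforms.
; BeginPlay and Tick are unused, and nothing in this file calls GeneratePlants.
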(fn `GeneratePlants`
  (params (SplineComp :type "SplineComponent Object Reference"))
  (bind _randomrotationrange (`self.RandomRotationRange`))
  (bind _returnvalue (`KismetMathLibrary.RandomFloatInRange` (`self.RandomScaleMin`) (`self.RandomScaleMax`)))
  (for _index (range (+ (`KismetMathLibrary.FFloor` (/ (`SplineComponent.GetSplineLength` SplineComp) (`self.SpawnSpacing`))) 1))
    (bind _returnvalue_2 (* _index (`self.SpawnSpacing`)))
    (`InstancedStaticMeshComponent.AddInstance` (`self.InstancedMeshComponent`) (`KismetMathLibrary.MakeTransform` (`SplineComponent.GetLocationAtDistanceAlongSpline` SplineComp _returnvalue_2 "World") (`KismetMathLibrary.ComposeRotators` (`KismetMathLibrary.Conv_VectorToRotator` (`SplineComponent.GetLocationAtDistanceAlongSpline` SplineComp _returnvalue_2 "World")) (`KismetMathLibrary.MakeRotator` 0.0 0.0 (`KismetMathLibrary.RandomFloatInRange` (* _randomrotationrange -1.0) _randomrotationrange))) (`KismetMathLibrary.MakeVector` _returnvalue _returnvalue _returnvalue)) false))
  (return))